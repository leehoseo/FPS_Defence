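; BP_ArmingCapsule is a gimmick actor whose capsule opens while a character is inside its trigger box and closes again when one leaves.
; Box overlap plays or reverses the MoveCapsule timeline, filtered to Character actors.
; The timeline's CapsuleOpen track, scaled by spline length, moves and rotates the Cylinder along the Spline, so the spline defines the opening path.
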(event OnComponentBeginOverlap(Box)
  (params (OverlappedComponent :type Primitive%20Component%20Object%20Reference) (OtherActor :type Actor%20Object%20Reference) (OtherComp :type Primitive%20Component%20Object%20Reference) (OtherBodyIndex :type Integer) (bFromSweep :type Boolean) (SweepResult :type Hit%20Result%20Structure%20%28by%20ref%29))
  (bind _spline (Variables|Default|GetSpline))
  (Utilities|Casting|CastToCharacter OtherActor)
  (bind _capsuleopen (Timeline|MoveCapsule Play)
    (:Update
      (Transformation|SetWorldLocation (Variables|Default|GetCylinder) (Spline|GetLocationatDistanceAlongSpline _spline (* _capsuleopen (Spline|GetSplineLength (Variables|Default|GetSpline))) "World") false false)
      (Transformation|SetRelativeRotation (Variables|Default|GetCylinder) (Spline|GetRotationatDistanceAlongSpline _spline (* _capsuleopen (Spline|GetSplineLength (Variables|Default|GetSpline))) "Local") false false))))

(event OnComponentEndOverlap(Box)
  (params (OverlappedComponent :type Primitive%20Component%20Object%20Reference) (OtherActor :type Actor%20Object%20Reference) (OtherComp :type Primitive%20Component%20Object%20Reference) (OtherBodyIndex :type Integer))
  (bind _spline (Variables|Default|GetSpline))
  (Utilities|Casting|CastToCharacter OtherActor)
  (bind _capsuleopen (Timeline|MoveCapsule Reverse)
    (:Update
      (Transformation|SetWorldLocation (Variables|Default|GetCylinder) (Spline|GetLocationatDistanceAlongSpline _spline (* _capsuleopen (Spline|GetSplineLength (Variables|Default|GetSpline))) "World") false false)
      (Transformation|SetRelativeRotation (Variables|Default|GetCylinder) (Spline|GetRotationatDistanceAlongSpline _spline (* _capsuleopen (Spline|GetSplineLength (Variables|Default|GetSpline))) "Local") false false))))

(fn ConstructionScript)