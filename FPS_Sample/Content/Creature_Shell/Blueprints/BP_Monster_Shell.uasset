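; BP_Monster_Shell is the Shell creature's monster Blueprint, reporting which characters enter or leave its two attack hitboxes.
; Begin and end overlaps on LeftAttackBox and RightAttackBox cast self to MonsterCharacter and the other actor to CommonCharacter, then call OnOverlappedCharacter or OffOverlappedCharacter.
; The graph holds no damage logic; BeginPlay, Tick and ActorBeginOverlap are disabled placeholders, and the construction script only calls its parent.
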(event OnComponentBeginOverlap(LeftAttackBox)
  (params (OverlappedComponent :type Primitive%20Component%20Object%20Reference) (OtherActor :type Actor%20Object%20Reference) (OtherComp :type Primitive%20Component%20Object%20Reference) (OtherBodyIndex :type Integer) (bFromSweep :type Boolean) (SweepResult :type Hit%20Result%20Structure%20%28by%20ref%29))
  (Utilities|Casting|CastToMonsterCharacter self)
  (bind _ascommon_character (Utilities|Casting|CastToCommonCharacter OtherActor))
  (Class|MonsterCharacter|OnOverlappedCharacter _ascommon_character))

(event OnComponentBeginOverlap(RightAttackBox)
  (params (OverlappedComponent :type Primitive%20Component%20Object%20Reference) (OtherActor :type Actor%20Object%20Reference) (OtherComp :type Primitive%20Component%20Object%20Reference) (OtherBodyIndex :type Integer) (bFromSweep :type Boolean) (SweepResult :type Hit%20Result%20Structure%20%28by%20ref%29))
  (Utilities|Casting|CastToMonsterCharacter self)
  (bind _ascommon_character (Utilities|Casting|CastToCommonCharacter OtherActor))
  (Class|MonsterCharacter|OnOverlappedCharacter _ascommon_character))

(event OnComponentEndOverlap(RightAttackBox)
  (params (OverlappedComponent :type Primitive%20Component%20Object%20Reference) (OtherActor :type Actor%20Object%20Reference) (OtherComp :type Primitive%20Component%20Object%20Reference) (OtherBodyIndex :type Integer))
  (Utilities|Casting|CastToMonsterCharacter self)
  (bind _ascommon_character (Utilities|Casting|CastToCommonCharacter OtherActor))
  (Class|MonsterCharacter|OffOverlappedCharacter _ascommon_character))

(event OnComponentEndOverlap(LeftAttackBox)
  (params (OverlappedComponent :type Primitive%20Component%20Object%20Reference) (OtherActor :type Actor%20Object%20Reference) (OtherComp :type Primitive%20Component%20Object%20Reference) (OtherBodyIndex :type Integer))
  (Utilities|Casting|CastToMonsterCharacter self)
  (bind _ascommon_character (Utilities|Casting|CastToCommonCharacter OtherActor))
  (Class|MonsterCharacter|OffOverlappedCharacter _ascommon_character))

(event EventBeginPlay
  (|CallParentFunction) ; 지금 이 노드는 비활성 상태입니다. \n핀을 끌어서 다른 노드를 연결하면 활성화됩니다.
)

(event Collision|EventActorBeginOverlap
  (params (OtherActor :type Actor%20Object%20Reference))
  (|CallParentFunction OtherActor) ; 지금 이 노드는 비활성 상태입니다. \n핀을 끌어서 다른 노드를 연결하면 활성화됩니다.
)

(event EventTick
  (params (DeltaSeconds :type Float%20%28single-precision%29))
  (|CallParentFunction DeltaSeconds) ; 지금 이 노드는 비활성 상태입니다. \n핀을 끌어서 다른 노드를 연결하면 활성화됩니다.
)

(fn ConstructionScript
  (|CallParentFunction))